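; BP_SpellStone is a collectable runestone that spins in the level and is picked up when something overlaps its box.
; On overlap it plays a pickup sound at the player pawn and increments the SpellStones count in the GameProgress game instance.
; It then calls HideCollected with its ID, which hides the mesh and indicator sprite and disables collision when the ID matches.
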(event OnComponentBeginOverlap(Box)
  (params (OverlappedComponent :type Primitive%20Component%20Object%20Reference) (OtherActor :type Actor%20Object%20Reference) (OtherComp :type Primitive%20Component%20Object%20Reference) (OtherBodyIndex :type Integer) (bFromSweep :type Boolean) (SweepResult :type Hit%20Result%20Structure%20%28by%20ref%29))
  ;[1 1 1] Spellstone collection mechanics
  (Audio|PlaySoundatLocation "/Game/Audio/Collectibles/MS_Pickup_Runestone.MS_Pickup_Runestone" (Transformation|GetActorLocation (Game|Player|GetPlayerPawn 0)) "0, 0, 0" 1.0 1.0 0.0 0 0 0 0)
  (bind _asgame_progress (Utilities|Casting|CastToGameProgress (Game|GetGameInstance)))
  (Variables|/Game/GameProgress.GameProgress_C|SetSpellStones _asgame_progress (+ (Variables|/Game/GameProgress.GameProgress_C|GetSpellStones _asgame_progress) 1))
  (Utilities|Casting|CastToGameProgress (Game|GetGameInstance))
  (CallFunction|HideCollected self (Variables|Default|GetID)))

(event Custom|HideCollected
  (params (ID_SpellStone :type Integer))
  ;[1 1 1] Hide Item when collected and Set no collision
  (if (== ID_SpellStone (Variables|Default|GetID))
    (Rendering|SetVisibility (Variables|Default|GetRuneStone) false false)
    (Collision|SetCollisionEnabled (Variables|Default|GetBox) "NoCollision")
    (Rendering|SetVisibility (Variables|Default|GetItemIndicatorSprite) false false)))

(event EventTick
  (params (DeltaSeconds :type Float%20%28single-precision%29))
  (Transformation|AddLocalRotation (Variables|Default|GetRuneStone) "0,5.000000, 0" false false))

(fn ConstructionScript)